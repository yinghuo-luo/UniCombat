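; BPC_Combat is a player controller Blueprint for the combat framework that sets up local input and UI when play begins.
; On BeginPlay, if it is the local player controller, it adds the default, mouse look and GAS Atlas Enhanced Input mapping contexts at equal priority.
; It then asks the UI root subsystem to ensure the UI exists, a step that runs outside the local-controller check.
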(event `self.ReceiveBeginPlay`
  (`|ExecutionSequence`
    (:`then_0`
      (if (`self.IsLocalPlayerController`)
        (`EnhancedInputSubsystemInterface.AddMappingContext` (subsystem `EnhancedInputLocalPlayerSubsystem`) "/Game/UniCombat/Input/IMC_Default.IMC_Default" 0 (struct))
        (`EnhancedInputSubsystemInterface.AddMappingContext` (subsystem `EnhancedInputLocalPlayerSubsystem`) "/Game/UniCombat/Input/IMC_MouseLook.IMC_MouseLook" 0 (struct))
        (`EnhancedInputSubsystemInterface.AddMappingContext` (subsystem `EnhancedInputLocalPlayerSubsystem`) "/Game/UniCombat/Input/IMC_GAS_Atlas.IMC_GAS_Atlas" 0 (struct))))
    (:`then_1`
      (`UIRootSubsystem.EnsureUI` (subsystem `UIRootSubsystem`)))))

(fn `UserConstructionScript`)